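; Socket API Blueprint that exposes events for controlling rain, day length and fetch quest creation.
; SetRainIntensity forwards to RainManager, and SetDayLength writes the in-game day length in minutes to GoodSky.
; CreateFetchQuest only stores the item count and a flag, which Tick consumes to call QuestManager, because quest creation must run on the game thread.
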(event `self.ReceiveTick`
  (params (DeltaSeconds :type "Float (single-precision)"))
  (if (`self.ShouldCreateFetchQuest`)
    (`/Game/KyleBlueprints/Quest/Quest_Manager.Create Quest` (`self.Quest Manager`) (`self.FetchQuestNumItems`))
    (set `self.ShouldCreateFetchQuest` false)))

(event `self.SetRainIntensity`
  (params (rain :type "Float (single-precision)"))
  (`/Game/KyleBlueprints/Rain/RainManager.Set Intensity` (`self.Rain Manager`) rain))

(event `self.SetDayLength`
  (params (minutes :type "Float (single-precision)"))
  (set `/Game/GoodSky/Blueprint/BP_GoodSky.└ How long is a day in the game? ( Unit : Minute )` minutes (`self.Good Sky`)))

(event `self.CreateFetchQuest`
  (params (items :type Integer))
  ;[1 1 1] Create Fetch Quest - Must be done in game thread.  See Event Tick
  (set `self.ShouldCreateFetchQuest` true)
  (set `self.FetchQuestNumItems` items))

(fn `UserConstructionScript`)